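; Deprecated enemy base actor that watches for the player and switches into combat once it spots them.
; A random tick slot chosen at BeginPlay staggers sight checks across instances, avoiding a trace every frame.
; The check line-traces on Visibility, ignoring other enemies, and sets InCombat on a close-range hit.
; The player controller is a placeholder target marked for replacement, and CombatMode is an empty stub that replaces sight checks once in combat.
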(event `self.ReceiveBeginPlay`
  ;[1 1 1] Psudo-distrubtation for update passes
  (set `self.TickToUpdate` (`KismetMathLibrary.RandomIntegerInRange` 1 5)))

(event `self.ReceiveTick`
  (params (DeltaSeconds :type "Float (single-precision)"))
  ;[1 1 1] Only performing targeting raycheck if the update tick matches. Ticker pauses while in combat mode.
  (if (`self.InCombat?`)
    (`self.CombatMode`)
    (else
      (bind _result (`/Engine/EditorBlueprintResources/StandardMacros.IncrementInt` (`self.TickPass`))
        (:`  `
          (if (> _result 5)
            (set `self.TickPass` 0)
            (elif (== (`self.TickToUpdate`) (`self.TickPass`))
              (`self.Update_PlayerSight`))))))))

(event `Update_PlayerSight`
  (bind _returnvalue (`GameplayStatics.GetPlayerController` 0))
  (bind _outactors (`GameplayStatics.GetAllActorsOfClass` "Deprecated_Enemy_Core_C"))
  (bind _outhit (`KismetSystemLibrary.LineTraceSingle` (`self.K2_GetActorLocation`) (`self.K2_GetActorLocation` (`GameplayStatics.GetPlayerController` 0)) "TraceTypeQuery1" false _outactors "ForDuration" true (struct :`R` 1.0 :`A` 1.0) (struct :`G` 1.0 :`A` 1.0) 1.0))
  (if (and (== (`.HitActor` (`GameplayStatics.BreakHitResult` _outhit)) _returnvalue) (< (`self.GetDistanceTo` self _returnvalue) 500.0))
    (set `self.InCombat?` true)
    (`KismetSystemLibrary.PrintString` "PLAYER SPOTTED. ATTACKING!")))

(event `CombatMode`)

(fn `UserConstructionScript`)