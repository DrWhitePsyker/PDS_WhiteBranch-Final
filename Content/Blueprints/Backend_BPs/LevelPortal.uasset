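; LevelPortal is a spinning portal actor that ends the current level when the player pawn overlaps it.
; On overlap it prints a debug message, reopens the current level by name, then increments LevelNumber on BP_GameInfoInstance, so the count persists across the reload.
; Tick advances the actor's yaw by a fixed step each frame, so spin speed depends on frame rate.
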(event `self.ReceiveActorBeginOverlap`
  (params (OtherActor :type "Actor Object Reference"))
  (if (== OtherActor (`GameplayStatics.GetPlayerPawn` 0))
    (`KismetSystemLibrary.PrintString` "LEVEL ENDING")
    (bind _returnvalue (`GameplayStatics.GetCurrentLevelName` true))
    (`GameplayStatics.OpenLevel` (`KismetStringLibrary.Conv_StringToName` _returnvalue))
    (bind _asbp_game_info_instance (cast `/Game/Blueprints/Backend_BPs/BP_GameInfoInstance` (`GameplayStatics.GetGameInstance`)))
    (`/Engine/EditorBlueprintResources/StandardMacros.IncrementInt` (`/Game/Blueprints/Backend_BPs/BP_GameInfoInstance.Level Number` _asbp_game_info_instance))))

(event `self.ReceiveTick`
  (params (DeltaSeconds :type "Float (single-precision)"))
  (bind (_returnvalue_roll _returnvalue_pitch _returnvalue_yaw) (`KismetMathLibrary.BreakRotator` (`self.K2_GetActorRotation`)))
  (`self.K2_SetActorRotation` (`KismetMathLibrary.MakeRotator` 0.0 0.0 (+ _returnvalue_yaw 1.0))))

(fn `UserConstructionScript`)