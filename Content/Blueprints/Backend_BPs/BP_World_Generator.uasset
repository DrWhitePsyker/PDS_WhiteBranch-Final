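; Procedural level generator that builds a straight run of random rooms on BeginPlay, with the room count scaling with the GameInstance's level number.
; RoomSpawn recursively picks rows from RoomDatabase, using each room's length to place it end-to-end along negative X and record its position.
; It then spawns the level portal in the last room plus end walls, and EnemySpawning scatters random numbers of enemies on navigable points around each room.
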(event `self.ReceiveBeginPlay`
  (bind _asbp_game_info_instance (cast `/Game/Blueprints/Backend_BPs/BP_GameInfoInstance` (`GameplayStatics.GetGameInstance`))
    (:`then`
      (bind _output_get (set `self.LevelNumber` (`/Game/Blueprints/Backend_BPs/BP_GameInfoInstance.Level Number` _asbp_game_info_instance))))
    (:`CastFailed`
      (`KismetSystemLibrary.PrintString` "games instance cast failed?")
      (`KismetSystemLibrary.PrintString` "Assume level 1")))
  (set `self.Rooms remaining` (+ _output_get 5))
  (`KismetSystemLibrary.PrintString` "SPAWN START ROOM")
  (`self.RoomSpawn`))

(event `RoomSpawn`
  (bind _spawnpostion (`self.spawnpostion`))
  (if (> (`self.Rooms remaining`) 0)
    (bind _output_get (set `self.Level ID rolled` (`KismetMathLibrary.RandomIntegerInRange` 1 4)))
    (bind _returnvalue (`|GetDataTableRow` "/Game/Blueprints/Enviro_BP/Rooms/RoomDatabase.RoomDatabase" (`KismetStringLibrary.Conv_StringToName` (`KismetStringLibrary.Conv_IntToString` _output_get)))
      (:`then`
        (bind (_roomid _roomlength) (break `/Game/Blueprints/Enviro_BP/Rooms/RoomStruct` _returnvalue))
        (bind _output_get_2 (set `self.SizeToShift` (/ _roomlength 2)))
        (bind _output_get_3 (set `self.X point` (+ (`self.X point`) _output_get_2)))
        (bind _output_get_4 (set `self.spawnpostion` (`KismetMathLibrary.MakeTransform` (`KismetMathLibrary.MakeVector` (`KismetMathLibrary.Conv_IntToDouble` (* _output_get_3 -1))))))
        (`|SpawnActorFromClass` _roomid _output_get_4 "Undefined" "OverrideRootScale" null null)
        (bind _output_get_5 (set `self.PrevSpawnPostion` _output_get_4))
        (`KismetArrayLibrary.Array_Add` (`self.SpawnPositions`) _output_get_5)
        (set `self.X point` (+ (`self.X point`) (`self.SizeToShift`)))
        (`/Engine/EditorBlueprintResources/StandardMacros.DecrementInt` (`self.Rooms remaining`)
          (:`  `
            (`self.RoomSpawn`))))
      (:`RowNotFound`
        (`KismetSystemLibrary.PrintString` "what the fuck")))
    (else
      (`|SpawnActorFromClass` "/Game/Blueprints/Backend_BPs/LevelPortal.LevelPortal_C" (`self.PrevSpawnPostion`) "Undefined" "OverrideRootScale" null null)
      (`|SpawnActorFromClass` "/Game/Blueprints/Enviro_BP/End_walls.End_walls_C" (`KismetMathLibrary.MakeTransform` (`KismetMathLibrary.MakeVector` (- (.x (.location _spawnpostion)) (`KismetMathLibrary.Conv_IntToDouble` (`self.SizeToShift`))) (.y (.location _spawnpostion)) (.z (.location _spawnpostion)))) "Undefined" "OverrideRootScale" null null)
      (`self.Enemy Spawning`))))

(event `Enemy Spawning`
  (for (_array_element _array_index) (`self.SpawnPositions`)
    (`KismetSystemLibrary.PrintString` (`KismetStringLibrary.Conv_IntToString` _array_index))
    (for _ (range (+ (`KismetMathLibrary.RandomIntegerInRange` 1 9) 1))
      (`|SpawnActorFromClass` "/Game/Blueprints/Enemy_BPs/Enemy_Core.Enemy_Core_C" (`KismetMathLibrary.MakeTransform` (`NavigationSystemV1.K2_GetRandomLocationInNavigableRadius` (.location _array_element) 500.0 null null)) "AdjustIfPossibleButAlwaysSpawn" "OverrideRootScale" null null)))
  (`KismetSystemLibrary.PrintString` "enemies spawned"))

(fn `UserConstructionScript`)