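; Bullet_Parent is a projectile Blueprint, apparently a base for bullets, that flies forward and damages what it overlaps.
; Tick moves it with a swept offset along its forward vector, scaling X and Y by Velocity and delta time but leaving Z unscaled.
; On overlap it ignores its Instigator and Bullet_Parent, otherwise sends a TakeDamage message of 1 and destroys itself, with debug prints throughout.
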(event `self.ReceiveBeginPlay`
  (`KismetSystemLibrary.PrintString` "BULLET AWAKENS"))

(event `self.ReceiveActorBeginOverlap`
  (params (OtherActor :type "Actor Object Reference"))
  (bind _hitactor (`self.HitActor`))
  (set `self.HitActor` OtherActor)
  (`KismetSystemLibrary.PrintString` "colision detected")
  (`KismetSystemLibrary.PrintString` (`KismetSystemLibrary.GetObjectName` (`self.HitActor`)))
  (if (or (== (`self.Instigator`) _hitactor) (== _hitactor "Bullet_Parent"))
    (`KismetSystemLibrary.PrintString` "Touch is self or parent, ignoring")
    (else
      (bind _asactor (cast `Actor` (`self.HitActor`))
        (:`then`
          (message `/Game/Blueprints/Backend_BPs/Bullet_Impact_Handler.Take_Damage` _asactor 1))
        (:`CastFailed`
          (`KismetSystemLibrary.PrintString` "cast to object failed. Killing bullet.")))
      (`self.K2_DestroyActor`))))

(event `self.ReceiveTick`
  (params (DeltaSeconds :type "Float (single-precision)"))
  (bind (_returnvalue_x _returnvalue_y _returnvalue_z) (`KismetMathLibrary.BreakVector` (`self.GetActorForwardVector`)))
  (bind _returnvalue (* (`self.Velocity`) DeltaSeconds))
  (`self.K2_AddActorWorldTransform` (`KismetMathLibrary.MakeTransform` (`KismetMathLibrary.MakeVector` (* _returnvalue_x _returnvalue) (* _returnvalue_y _returnvalue) _returnvalue_z)) true))

(fn `UserConstructionScript`)