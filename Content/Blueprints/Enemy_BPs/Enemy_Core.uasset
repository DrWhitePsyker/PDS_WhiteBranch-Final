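; Prototype enemy pawn that spots the player and holds a preferred distance in combat.
; It registers with Enemy_Manager on spawn, and its sight event line-traces to a nearby player to latch InCombat.
; Tick moves it to a cached standoff point, recalculated when drift exceeds ShuffleSpace, with debug draws and a placeholder ChargeLock branch.
; Any damage just flags IsDead, leaving death handling to the manager.
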(event `self.ReceiveBeginPlay`
  (bind _outactors (`GameplayStatics.GetAllActorsOfClass` "/Game/Blueprints/Enemy_BPs/Enemy_Manager.Enemy_Manager_C"))
  (bind _output_get (set `self.Enemy Manager Pointer` (`|GetArrayItem` _outactors)))
  (if (`KismetSystemLibrary.IsValid` _output_get)
    (bind _asenemy_manager (cast `/Game/Blueprints/Enemy_BPs/Enemy_Manager` (`self.Enemy Manager Pointer`)))
    (`/Game/Blueprints/Enemy_BPs/Enemy_Manager.FeedToUpdateArray` _asenemy_manager self)
    (bind _outactors_2 (`GameplayStatics.GetAllActorsOfClass` "/Game/Blueprints/Player_BPs/BP_Character.BP_Character_C"))
    (set `self.Player Pointer` (`|GetArrayItem` _outactors_2))
    (else
      (`KismetSystemLibrary.PrintString` (`KismetStringLibrary.Concat_StrStr` (`KismetStringLibrary.Concat_StrStr` "ERROR IN: " (`KismetSystemLibrary.GetDisplayName` self)) "  # enemy manager pointer invalid. Is there an enemy manager active?"))
      (`self.K2_DestroyActor`))))

(event `Update_PlayerSight`
  (bind (_returnvalue_x _returnvalue_y _returnvalue_z) (`KismetMathLibrary.BreakVector` (`self.K2_GetActorLocation`)))
  (if (< (`self.GetDistanceTo` self (`self.Player Pointer`)) 1500.0)
    (bind _outactors (`GameplayStatics.GetAllActorsOfClass` "Enemy_Core_C"))
    (bind _outhit (`KismetSystemLibrary.LineTraceSingle` (`KismetMathLibrary.MakeVector` _returnvalue_x _returnvalue_y (+ _returnvalue_z 50.0)) (`SceneComponent.K2_GetComponentLocation` (`/Game/Blueprints/Player_BPs/BP_Character.Character` (`self.Player Pointer`))) "TraceTypeQuery1" false _outactors "ForDuration" true (struct :`R` 1.0 :`A` 1.0) (struct :`G` 1.0 :`A` 1.0) 0.1))
    (if (== (`.HitActor` (`GameplayStatics.BreakHitResult` _outhit)) (`self.Player Pointer`))
      (set `self.InCombat?` true)
      (`KismetSystemLibrary.PrintString` "PLAYER SPOTTED. ATTACKING!"))))

(event `self.ReceiveTick`
  (params (DeltaSeconds :type "Float (single-precision)"))
  (bind _prefered_distance (`self.Prefered distance`))
  (bind (_returnvalue_x _returnvalue_y) (`KismetMathLibrary.BreakVector` (`KismetMathLibrary.GetDirectionUnitVector` (`self.K2_GetActorLocation` self) (`self.K2_GetActorLocation` (`self.Player Pointer`)))))
  (bind _returnvalue (+ (`self.K2_GetActorLocation` (`self.Player Pointer`)) (`KismetMathLibrary.MakeVector` (* (* _returnvalue_x _prefered_distance) -1.0) (* (* _returnvalue_y _prefered_distance) -1.0))))
  (if (`self.InCombat?`)
    (if (`self.ChargeLock?`)
      (`KismetSystemLibrary.PrintString` "SWIGGITY SWOOTY ")
      (else
        (if (not (`self.HasPath?`))
          (set `self.Precalc point` _returnvalue)
          (set `self.HasPath?` true))
        (`KismetSystemLibrary.DrawDebugPoint` (`self.Precalc point`) 5.0 (struct :`R` 0.4375 :`A` 1.0) 0.1)
        (`KismetSystemLibrary.DrawDebugPoint` _returnvalue 5.0 (struct :`G` 0.055574 :`B` 0.739583 :`A` 1.0) 0.1)
        (if (> (`KismetMathLibrary.Abs` (`KismetMathLibrary.Vector_Distance` (`self.Precalc point`) _returnvalue)) (`self.Shuffle space`))
          (set `self.HasPath?` false)
          (else
            (`|AIMoveTo` self (`self.Precalc point`) null 5.0 true
              (:`then`
                (set `self.IsAttacking?` (> (`KismetMathLibrary.Abs` (`KismetMathLibrary.Vector_Distance` (`self.Precalc point`) (`self.K2_GetActorLocation`))) 5.0))))))))))

(event `/Game/Blueprints/Backend_BPs/Bullet_Impact_Handler.Take_Damage`
  (params (DamageValue :type Integer))
  ;[1 1 1] This would use a health-system to check if the damage dealt has brough the health value below 0 before destroying it, but this is ignored for the prototype. The enemy manager handles this
  (set `self.IsDead?` true))

(fn `UserConstructionScript`)