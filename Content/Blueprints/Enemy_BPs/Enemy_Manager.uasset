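; Enemy manager that time-slices enemy updates across frames to spread out their sight and pathfinding cost.
; FeedToUpdateArray deals incoming enemies round-robin into a nested array of groups, using a wrapping counter.
; Each Tick processes one group, destroying and removing dead Enemy_Core actors and calling UpdatePlayerSight on those out of combat.
; A second wrapping counter advances the group each frame, so each enemy updates once per cycle.
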(event `FeedToUpdateArray`
  (params (EnemyNeedingSorting :type "Actor Object Reference"))
  ;[1 1 1] This system sorts the enemies into 18 groups. This allows us to spread out the number of path finding requests over 18 frames.
  (`KismetArrayLibrary.Array_Add` (`.ArrayX_4_F523468849DDE91D66375189325E2D77` (break `/Game/Blueprints/Backend_BPs/ActorArrayStruct` (`|GetArrayItem` (`self.EnemyUpdateArrayY`) (`self.Sorting Pass`)))) EnemyNeedingSorting)
  (bind _result (`/Engine/EditorBlueprintResources/StandardMacros.IncrementInt` (`self.Sorting Pass`))
    (:`  `
      (if (> _result 18)
        (set `self.Sorting Pass` 0)))))

(event `self.ReceiveTick`
  (params (DeltaSeconds :type "Float (single-precision)"))
  (bind _arrayx (break `/Game/Blueprints/Backend_BPs/ActorArrayStruct` (`|GetArrayItem` (`self.EnemyUpdateArrayY`) (`self.TickPass`))))
  ;[1 1 1] THIS NEEDS PATCHING FOR ENEMY CORE CHILDREN
  (for (_array_element _array_index) _arrayx
    (bind _asenemy_core (cast `/Game/Blueprints/Enemy_BPs/Enemy_Core` _array_element)
      (:`then`
        ;[1 1 1] DARE YOU ENTER MY SPAGETTI FORTRESS OF PERPETUAL CONFUSION?!
        (if (`/Game/Blueprints/Enemy_BPs/Enemy_Core.IsDead?` _asenemy_core)
          (`self.K2_DestroyActor` _asenemy_core)
          (`KismetArrayLibrary.Array_Remove` _arrayx _array_index)
          (elif (not (`/Game/Blueprints/Enemy_BPs/Enemy_Core.InCombat?` _asenemy_core))
            (`/Game/Blueprints/Enemy_BPs/Enemy_Core.Update_PlayerSight` _asenemy_core))))
      (:`CastFailed`
        (`KismetSystemLibrary.PrintString` "EnemyManager: Pass object is not enemy_core?"))))
  (bind _result (`/Engine/EditorBlueprintResources/StandardMacros.IncrementInt` (`self.TickPass`))
    (:`  `
      (if (> _result 18)
        (set `self.TickPass` 0)))))

(fn `UserConstructionScript`)