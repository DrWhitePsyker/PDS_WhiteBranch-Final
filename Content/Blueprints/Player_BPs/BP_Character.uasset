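; BP_Character is the player character, with world-axis movement, yaw turning, sprinting and shooting.
; On BeginPlay it spawns a BP_Camera offset behind and above, pitched steeply down and targeting itself.
; Input switches walk speed for running and spawns BP_Bullet at the actor's transform.
; TakeDamage decrements and prints Health, but its overlap trigger is unwired, as is the leftover Sprint function's logic.
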(event `self.ReceiveBeginPlay`
  (bind (_returnvalue_x _returnvalue_y _returnvalue_z) (`KismetMathLibrary.BreakVector` (`self.K2_GetActorLocation`)))
  ;[1 1 1] Character & Camera Spawn
  (bind _returnvalue (`|SpawnActorFromClass` "/Game/Blueprints/Player_BPs/BP_Camera.BP_Camera_C" (`KismetMathLibrary.MakeTransform` (`KismetMathLibrary.MakeVector` (- _returnvalue_x 200.0) _returnvalue_y (+ _returnvalue_z 500.0)) (struct :`Pitch` -80.0)) "Undefined" "OverrideRootScale" null null))
  (set `/Game/Blueprints/Player_BPs/BP_Camera.playertarget` self _returnvalue)
  (`self.EnableInput` (`GameplayStatics.GetPlayerController` 0))
  (set `CharacterMovementComponent.MaxWalkSpeed` (`self.Walk Speed`) (`self.CharacterMovement`))
  (set `self.Health` (`self.Health`)))

(event `InputAction|Shoot`
  (params (Key :type "Key Structure"))
  ;[1 1 1] Shoot Functionality
  (:`Pressed`
    (`|SpawnActorFromClass` "/Game/Blueprints/Backend_BPs/BP_Bullet.BP_Bullet_C" (`self.GetTransform`) "Undefined" "OverrideRootScale" null self)))

(event `InputAxis|Turn`
  (params (AxisValue :type "Float (single-precision)"))
  ;[1 1 1] Movement Funtionality
  (`self.AddControllerYawInput` AxisValue))

(event `InputAxis|MoveForward`
  (params (AxisValue :type "Float (single-precision)"))
  ;[1 1 1] Movement Funtionality
  (`self.AddMovementInput` (1.0 0.0 0.0) AxisValue true))

(event `InputAxis|Moveright`
  (params (AxisValue :type "Float (single-precision)"))
  ;[1 1 1] Movement Funtionality
  (`self.AddMovementInput` (0.0 1.0 0.0) AxisValue true))

(event `InputAction|Run`
  (params (Key :type "Key Structure"))
  (bind _charactermovement (`self.CharacterMovement`))
  (:`Pressed`
    (set `CharacterMovementComponent.MaxWalkSpeed` (`self.Sprint Speed`) _charactermovement))
  (:`Released`
    (set `CharacterMovementComponent.MaxWalkSpeed` (`self.Walk Speed`) _charactermovement)))

(event `self.ReceiveActorBeginOverlap`
  (params (OtherActor :type "Actor Object Reference"))
  ;[1 1 1] Added 11/03/2020 - Take damage on overlap with pool
)

(fn `Sprint`)

(fn `TakeDamage`
  ;[1 1 1] Decrease health by 1 for each instance of damage taken
  (`/Engine/EditorBlueprintResources/StandardMacros.DecrementInt` (`self.Health`)
    (:`  `
      (`KismetSystemLibrary.PrintString` (`KismetStringLibrary.Conv_IntToString` (`self.Health`))))))

(fn `UserConstructionScript`)